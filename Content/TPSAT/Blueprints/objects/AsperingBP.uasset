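; AsperingBP is a spinning pickup that restores part of the story-adventure character's Drugs value.
; Tick steps the actor's roll and yaw each frame, without delta-time scaling, and zeroes its pitch.
; On Box overlap with BP_StoryAdv_Character, it adds a capped increment to Drugs, destroys itself and prints a string.
; If Drugs is already full, the pickup stays in the world.
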(event OnComponentBeginOverlap(Box)
  (params (OverlappedComponent :type Primitive%20Component%20Object%20Reference) (OtherActor :type Actor%20Object%20Reference) (OtherComp :type Primitive%20Component%20Object%20Reference) (OtherBodyIndex :type Integer) (bFromSweep :type Boolean) (SweepResult :type Hit%20Result%20Structure%20%28by%20ref%29))
  (bind _asbp_story_adv_character (Utilities|Casting|CastToBP_StoryAdv_Character OtherActor))
  (if (not (>= (Variables|/Game/TPSAT/Blueprints/Character/BP_StoryAdv_Character.BP_StoryAdv_Character_C|Getdrugs _asbp_story_adv_character) 1.0))
    (Variables|/Game/TPSAT/Blueprints/Character/BP_StoryAdv_Character.BP_StoryAdv_Character_C|Setdrugs _asbp_story_adv_character (Math|Float|Min(Float) (+ (Variables|/Game/TPSAT/Blueprints/Character/BP_StoryAdv_Character.BP_StoryAdv_Character_C|Getdrugs _asbp_story_adv_character) 0.2) 1.0))
    (Actor|DestroyActor)
    (Development|PrintString "Hello")))

(event EventBeginPlay)

(event Collision|EventActorBeginOverlap
  (params (OtherActor :type Actor%20Object%20Reference)))

(event EventTick
  (params (DeltaSeconds :type Float%20%28single-precision%29))
  (bind _returnvalue (Transformation|GetActorRotation))
  (bind (_roll _pitch _yaw) (Math|Rotator|BreakRotator _returnvalue))
  (Transformation|SetActorRelativeRotation (Math|Rotator|MakeRotator (+ _roll 1.0) 0.0 (+ _yaw 1.0))))

(fn ConstructionScript)